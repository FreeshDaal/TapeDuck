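; Quest-giver NPC that rates what the player brings and replies with dialogue from its quest struct.
; CheckFit counts acorn pickups or matches actor tags against thresholds, setting a star rating and spawning the quest item at three acorns or two-plus stars.
; ChangeDialogue selects lines by rating, and Speak steps through them using the player's dialogue camera and a widget.
; BeginPlay adds a hidden, slightly enlarged overlap mesh carrying the component tags.
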(event EventBeginPlay
  (Variables|Default|SetSpeechCurrent (.startdialogue (Variables|Default|GetMyQuest)))
  (bind _returnvalue (Game|AddComponentbyClass "/Script/Engine.StaticMeshComponent" false))
  (bind _output_get (Variables|Default|SetOverlappingMesh _returnvalue))
  (Components|StaticMesh|SetStaticMesh _output_get (Variables|Default|GetStatic%20Mesh))
  (Transformation|AttachComponentToComponent (Variables|Default|GetOverlappingMesh) 0 "None" "KeepRelative" "KeepRelative" "KeepRelative" true)
  (Transformation|SetRelativeScale3D (Variables|Default|GetOverlappingMesh) "1.150000,1.150000,1.150000")
  (Collision|SetCollisionResponsetoAllChannels (Variables|Default|GetOverlappingMesh) "ECR_Overlap")
  (Collision|SetCollisionResponsetoChannel (Variables|Default|GetOverlappingMesh) "ECC_Pawn" "ECR_Ignore")
  (Development|SetHiddeninGame (Variables|Default|GetOverlappingMesh) true false)
  (Collision|IgnoreActorwhenMoving (Variables|Default|GetOverlappingMesh) self true)
  (Class|PrimitiveComponent|SetMassOverrideinKg (Variables|Default|GetOverlappingMesh) "None" 1.0 true)
  (Variables|/Script/Engine.ActorComponent|SetComponentTags (Variables|Default|GetOverlappingMesh) (Variables|Default|GetComponent%20Tags))
  (Components|Animation|PlayAnimation (Variables|Default|GetSkeletalMesh) (Variables|Default|GetAnim) false))

(event Collision|EventActorBeginOverlap
  (params (OtherActor :type Actor%20Object%20Reference)))

(event EventTick
  (params (DeltaSeconds :type Float%20%28single-precision%29)))

(event EventCheckFit
  (params (From :type Interactable%20Object%20Object%20Reference))
  (CallFunction|RatingCheck From))

(event EventAnimation
  (CallFunction|StopPlayer))

(event EventCheckThresholds
  (params (Rating :type Integer) (TagsMatch :type Integer))
  (bind _returnvalue (Transformation|GetActorTransform))
  (bind _returnvalue_2 (Transformation|GetActorTransform))
  (if (== Rating -1)
    (bind _output_get (Variables|Default|SetAcorns (+ (Variables|Default|GetAcorns) 1)))
    (bind _structout (Utilities|Struct|SetmembersinQuest (Variables|Default|GetMyQuest) _output_get))
    (Variables|Default|SetMyQuest _structout)
    (if (>= _output_get 3)
      (Game|SpawnActorfromClass (.questitem (Variables|Default|GetMyQuest)) (Math|Transform|MakeTransform (+ (.location _returnvalue_2) "0.000000,0.000000,25.000000") (.rotation _returnvalue_2) (.scale _returnvalue_2)) "Undefined" "MultiplyWithRoot" 0 0)
      (else
        (CallFunction|ChangeDialogue :!label _label)
        (CallFunction|Speak)
        (Development|PrintString (Utilities|String|Append (Utilities|String|ToString(Integer) TagsMatch) " A"))))
    (else
      (if (< TagsMatch (.3threshold (Variables|Default|GetMyQuest)))
        (if (< TagsMatch (.2threshold (Variables|Default|GetMyQuest)))
          (if (< TagsMatch (.1threshold (Variables|Default|GetMyQuest)))
            (bind _structout_2 (Utilities|Struct|SetmembersinQuest (Variables|Default|GetMyQuest)))
            (Variables|Default|SetMyQuest _structout_2)
            (goto _label)
            (else
              (bind _structout_3 (Utilities|Struct|SetmembersinQuest (Variables|Default|GetMyQuest) 1))
              (Variables|Default|SetMyQuest _structout_3)
              (goto _label)))
          (else
            (bind _structout_4 (Utilities|Struct|SetmembersinQuest (Variables|Default|GetMyQuest) 2))
            (Variables|Default|SetMyQuest _structout_4)))
        (else
          (bind _structout_5 (Utilities|Struct|SetmembersinQuest (Variables|Default|GetMyQuest) 3))
          (Variables|Default|SetMyQuest _structout_5)))
      (Game|SpawnActorfromClass (.questitem (Variables|Default|GetMyQuest)) (Math|Transform|MakeTransform (+ (.location _returnvalue) "0.000000,0.000000,25.000000") (.rotation _returnvalue) (.scale _returnvalue)) "Undefined" "MultiplyWithRoot" 0 0)
      (goto _label))))

(fn ConstructionScript)

(fn Speak
  (if (== (Variables|Default|GetSpokenTo) 0)
    (bind _returnvalue (Actor|GetActorOfClass "/Game/PlayerBlueprint/BP_Player.BP_Player_C"))
    (Default|InitDialogueCam _returnvalue (.location (Transformation|GetActorTransform)) (Transformation|GetActorForwardVector) (Transformation|GetActorRightVector))
    (bind _returnvalue_2 (UserInterface|CreateWidget "/Game/UI/WB_Dialogue.WB_Dialogue_C" (Game|GetPlayerController 0)))
    (bind _output_get (Variables|Default|SetDialogue _returnvalue_2))
    (UserInterface|Viewport|AddtoPlayerScreen _output_get))
  (if (>= (Variables|Default|GetSpokenTo) (Utilities|Array|Length (Variables|Default|GetSpeechCurrent)))
    (bind _returnvalue_3 (Actor|GetActorOfClass "/Game/PlayerBlueprint/BP_Player.BP_Player_C"))
    (Default|EndDialogueCam _returnvalue_3)
    (CallFunction|ChangeDialogue)
    (Utilities|IsValid (Variables|Default|GetDialogue)
      (:Is%20Valid
        (Widget|RemovefromParent (Variables|Default|GetDialogue))))
    (else
      (Variables|/Script/UMG.TextBlock|SetText (Variables|/Game/UI/WB_Dialogue.WB_Dialogue_C|GetTextBlock_194 (Variables|Default|GetDialogue)) (Utilities|Text|ToText(String) (Utilities|Array|Get(acopy) (Variables|Default|GetSpeechCurrent) (Variables|Default|GetSpokenTo))))
      (Variables|Default|SetSpokenTo (Math|Integer|Clamp(Integer) (+ (Variables|Default|GetSpokenTo) 1) 0 (Utilities|Array|Length (Variables|Default|GetSpeechCurrent)))))))

(fn SaveDialogue
  (params (Say :type Array%20of%20Strings))
  (Variables|Default|SetSpeechCurrent Say)
  (CallFunction|Speak))

(fn ChangeDialogue
  (bind _myquest (Variables|Default|GetMyQuest))
  (switch int (.currentrating (Variables|Default|GetMyQuest))
    (:Default
      (Variables|Default|SetSpeechCurrent (.hint _myquest)))
    (:0
      (Variables|Default|SetSpeechCurrent (.0-star _myquest)))
    (:1
      (Variables|Default|SetSpeechCurrent (.1-star _myquest)))
    (:2
      (Variables|Default|SetSpeechCurrent (.2-star _myquest)))
    (:3
      (Variables|Default|SetSpeechCurrent (.3-star _myquest))))
  (Variables|Default|SetSpokenTo 0)
  (Development|PrintString (Utilities|String|ToString(Integer) (.currentrating (Variables|Default|GetMyQuest)))))

(fn RatingCheck
  (params (Attached :type Actor%20Object%20Reference))
  (bind _asacorn_pickup (Utilities|Casting|CastToAcornPickup Attached)
    (:then
      (CallFunction|CheckThresholds -1)
      (Actor|DestroyActor _asacorn_pickup))
    (:CastFailed
      (for _array_element (Variables|/Script/Engine.Actor|GetTags Attached)
        (for _array_element_2 (.tags (Variables|Default|GetMyQuest))
          (if (== _array_element_2 _array_element)
            (LocalVariables|SetMatchcount (+ (LocalVariables|GetMatchcount) 1)))))
      (CallFunction|CheckThresholds 0 (LocalVariables|GetMatchcount)))))

(fn ThresholdCheck
  (params (TagMatch :type Integer))
  (if (< TagMatch (.1threshold (Variables|Default|GetMyQuest)))
    (bind _structout (Utilities|Struct|SetmembersinQuest (Variables|Default|GetMyQuest)))
    (Variables|Default|SetMyQuest _structout)
    (elif (< TagMatch (.2threshold (Variables|Default|GetMyQuest)))
      (bind _structout_2 (Utilities|Struct|SetmembersinQuest (Variables|Default|GetMyQuest) 1))
      (Variables|Default|SetMyQuest _structout_2)
      (elif (< TagMatch (.3threshold (Variables|Default|GetMyQuest)))
        (bind _structout_3 (Utilities|Struct|SetmembersinQuest (Variables|Default|GetMyQuest) 2))
        (Variables|Default|SetMyQuest _structout_3)
        (else
          (bind _structout_4 (Utilities|Struct|SetmembersinQuest (Variables|Default|GetMyQuest) 3))
          (Variables|Default|SetMyQuest _structout_4)))))
  (CallFunction|ChangeDialogue)
  (CallFunction|Speak)
  (Development|PrintString (Utilities|String|ToString(Integer) (.currentrating (Variables|Default|GetMyQuest)))))

(fn StopPlayer)

(fn EchoType
  (return false))