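; QuestObject is an attachable quest item whose tag matches with the thing it attaches to earn a 0–3 star quest rating.
; On BeginPlay it adds a hidden, slightly enlarged overlap copy of its mesh and overrides the mesh's mass.
; AttachedToSomething counts matching actor tags, CheckThresholds sets the rating, and DialogueCheck saves matching dialogue to the NPC.
; On first meeting, DialogueCheck instead saves the start dialogue and applies the attach tag to the mesh.
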(event EventBeginPlay
  (bind _staticmesh (Variables|Default|GetStaticMesh))
  (bind _returnvalue (Game|AddComponentbyClass "/Script/Engine.StaticMeshComponent" false))
  (Components|StaticMesh|SetStaticMesh _returnvalue (Variables|/Script/Engine.StaticMeshComponent|GetStaticMesh _staticmesh))
  (Transformation|AttachComponentToComponent _returnvalue _staticmesh "None" "KeepRelative" "KeepRelative" "KeepRelative" true)
  (Transformation|SetRelativeScale3D _returnvalue "1.150000,1.150000,1.150000")
  (Collision|SetCollisionResponsetoAllChannels _returnvalue "ECR_Overlap")
  (Collision|SetCollisionResponsetoChannel _returnvalue "ECC_Pawn" "ECR_Ignore")
  (Development|SetHiddeninGame _returnvalue true false)
  (Collision|IgnoreActorwhenMoving _returnvalue self true)
  (Class|PrimitiveComponent|SetMassOverrideinKg (Variables|Default|GetStaticMesh) "None" 1e+02 true))

(event Collision|EventActorBeginOverlap
  (params (OtherActor :type Actor%20Object%20Reference)))

(event EventTick
  (params (DeltaSeconds :type Float%20%28single-precision%29)))

(fn ConstructionScript)

(fn CheckThresholds
  (params (MatchCount :type Integer))
  (if (< MatchCount (.1threshold (Variables|Default|GetMyQuest)))
    (bind _structout (Utilities|Struct|SetmembersinQuest (Variables|Default|GetMyQuest)))
    (Variables|Default|SetMyQuest _structout)
    (elif (< MatchCount (.2threshold (Variables|Default|GetMyQuest)))
      (bind _structout_2 (Utilities|Struct|SetmembersinQuest (Variables|Default|GetMyQuest) 1))
      (Variables|Default|SetMyQuest _structout_2)
      (elif (< MatchCount (.3threshold (Variables|Default|GetMyQuest)))
        (bind _structout_3 (Utilities|Struct|SetmembersinQuest (Variables|Default|GetMyQuest) 2))
        (Variables|Default|SetMyQuest _structout_3)
        (else
          (bind _structout_4 (Utilities|Struct|SetmembersinQuest (Variables|Default|GetMyQuest) 3))
          (Variables|Default|SetMyQuest _structout_4)))))
  (CallFunction|DialogueCheck))

(fn DialogueCheck
  (bind _myquest (Variables|Default|GetMyQuest))
  (bind _mynpc (Variables|Default|GetMyNPC))
  (if (Variables|Default|GetFirstMeeting)
    (Default|SaveDialogue (Variables|Default|GetMyNPC) (.startdialogue _myquest))
    (Variables|/Script/Engine.ActorComponent|SetComponentTags (Variables|Default|GetStaticMesh) (Variables|Default|GetAttachTag))
    (elif (Variables|Default|GetInitial%20Speak)
      (switch int (.currentrating _myquest)
        (:Default
          (Default|SaveDialogue _mynpc (.hint _myquest)))
        (:0
          (Default|SaveDialogue (Variables|Default|GetMyNPC) (.0-star _myquest)))
        (:1
          (Default|SaveDialogue (Variables|Default|GetMyNPC) (.1-star _myquest)))
        (:2
          (Default|SaveDialogue (Variables|Default|GetMyNPC) (.2-star _myquest)))
        (:3
          (Default|SaveDialogue (Variables|Default|GetMyNPC) (.3-star _myquest))))
      (Default|SaveDialogue _mynpc (.hint _myquest))
      (Variables|Default|SetInitial%20Speak false))))

(fn AttachedtoSomething
  (params (Attached%20Thing :type Actor%20Object%20Reference))
  (for _array_element (Variables|/Script/Engine.Actor|GetTags Attached%20Thing)
    (for _array_element_2 (Variables|Actor|GetTags self)
      (if (== _array_element_2 _array_element)
        (LocalVariables|Setmatchcount (+ (LocalVariables|Getmatchcount) 1)))))
  (CallFunction|CheckThresholds (LocalVariables|Getmatchcount)))

(fn EchoType
  (return false))