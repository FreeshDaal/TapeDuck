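; Base logic for a physics object that can be grabbed and attached to other objects.
; BeginPlay adds a hidden, 1.15x-scaled copy of its mesh as an overlap sensor.
; Grabbed detaches it and overrides mass to zero with CCD on; Attach2 restores mass and attaches it to a random overlapping "Attach"-tagged component's owner.
; An older socket-trace hologram snapping system remains, but its events are unwired.
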(event Custom|ProjectionSearch)

(event Custom|StartProjectionSearch)

(event Custom|ClearProjectionSearch)

(event Custom|Attach2
  (bind _touchingactors (Variables|Default|GetTouchingActors))
  (bind _staticmesh (Variables|Default|GetStaticMesh))
  (Class|PrimitiveComponent|SetUseCCD _staticmesh false "None")
  (Class|PrimitiveComponent|SetMassOverrideinKg _staticmesh "None" (Variables|Default|GetMass) true)
  (for _array_element (Class|PrimitiveComponent|GetOverlappingComponents (Variables|Default|GetOverlapMesh))
    (if (Components|ComponentHasTag _array_element "Attach")
      (if (not (Utilities|Array|ContainsItem (Actor|GetAttachedActors true true) (Components|GetOwner _array_element)))
        (Utilities|Array|Add (Variables|Default|GetTouchingActors) _array_element))))
  (if (Utilities|Array|IsNotEmpty _touchingactors)
    (Transformation|AttachActorToActor (Components|GetOwner (.OutItem (Utilities|Array|Random _touchingactors))) "None" "KeepWorld" "KeepWorld" "KeepWorld" true)
    (Utilities|Array|Clear (Variables|Default|GetTouchingActors))))

(event Custom|Grabbed
  (bind _staticmesh (Variables|Default|GetStaticMesh))
  (Class|PrimitiveComponent|SetUseCCD _staticmesh true "None")
  (Class|PrimitiveComponent|SetMassOverrideinKg _staticmesh "None" 0.0 true)
  (Collision|IgnoreActorwhenMoving (Variables|Default|GetStaticMesh) (Game|Player|GetPlayerPawn 0) true)
  (Transformation|DetachFromActor "KeepWorld" "KeepWorld" "KeepWorld"))

(event EventBeginPlay
  (bind _staticmesh (Variables|Default|GetStaticMesh))
  (bind _returnvalue (Game|AddComponentbyClass "/Script/Engine.StaticMeshComponent" false))
  (bind _output_get (Variables|Default|SetOverlapMesh _returnvalue))
  (Components|StaticMesh|SetStaticMesh _output_get (Variables|/Script/Engine.StaticMeshComponent|GetStaticMesh _staticmesh))
  (Transformation|AttachComponentToComponent (Variables|Default|GetOverlapMesh) _staticmesh "None" "KeepRelative" "KeepRelative" "KeepRelative" true)
  (Transformation|SetRelativeScale3D (Variables|Default|GetOverlapMesh) "1.150000,1.150000,1.150000")
  (Collision|SetCollisionResponsetoAllChannels (Variables|Default|GetOverlapMesh) "ECR_Overlap")
  (Collision|SetCollisionResponsetoChannel (Variables|Default|GetOverlapMesh) "ECC_Pawn" "ECR_Ignore")
  (Development|SetHiddeninGame (Variables|Default|GetOverlapMesh) true false)
  (Collision|IgnoreActorwhenMoving (Variables|Default|GetOverlapMesh) self true)
  (Class|PrimitiveComponent|SetMassOverrideinKg (Variables|Default|GetStaticMesh) "None" (Variables|Default|GetMass) true))

(event Collision|EventActorBeginOverlap
  (params (OtherActor :type Actor%20Object%20Reference)))

(event EventTick
  (params (DeltaSeconds :type Float%20%28single-precision%29)))

(fn ConstructionScript)

(fn ProjectionSearchCall
  (params (Final :type Boolean))
  (bind _returnvalue (Actor|GetComponentbyClass "/Game/PlayerBlueprint/BP_PickUpHologram.BP_PickUpHologram_C"))
  (bind _returnvalue_2 (Actor|GetComponentbyClass "/Game/PlayerBlueprint/BP_PickUpHologram.BP_PickUpHologram_C"))
  (bind _listofactors (LocalVariables|GetListofActors))
  (bind _staticmesh (Variables|Default|GetStaticMesh))
  (LocalVariables|SetClosest%20Distance 5e+01)
  (for _array_element (Variables|Default|GetSockets)
    (bind _detected (Default|Search _array_element))
    (for _array_element_2 _detected
      (Utilities|Array|AddUnique _listofactors _array_element_2))
    (if (Utilities|Array|IsEmpty _listofactors)
      (Utilities|IsValid _returnvalue_2
        (:Is%20Valid
          (Components|DestroyComponent _returnvalue_2)))
      (else
        (for _array_element_3 (LocalVariables|GetListofActors)
          (for _array_element_4 (Variables|Default|GetSockets)
            (bind _outhits (Class|KismetSystemLibrary|LineTraceMultiforObjects (Transformation|GetWorldLocation _array_element_4) (Transformation|GetActorLocation _array_element_3) (LocalVariables|GetTypes) false (LocalVariables|GetIgnore) "ForDuration" true "(R=1.000000,G=0.000000,B=0.000000,A=1.000000)" "(R=0.000000,G=1.000000,B=0.000000,A=1.000000)" 2.0))
            (for _array_element_5 _outhits
              (if (< (.distance _array_element_5) (LocalVariables|GetClosest%20Distance))
                (bind _output_get (LocalVariables|SetClosest%20Distance (.distance _array_element_5)))
                (bind _output_get_2 (LocalVariables|SetChosenActor _array_element_3))
                (LocalVariables|SetChosenSocket _array_element_4)
                (LocalVariables|SetData (Utilities|Struct|MakeAttachData (.impactpoint _array_element_5) (.impactnormal _array_element_5) _output_get_2 _output_get (Actor|GetComponentbyClass "/Game/PlayerBlueprint/BP_PickUpHologram.BP_PickUpHologram_C")))))))
        (if Final
          (Utilities|IsValid _returnvalue
            (:Is%20Valid
              (Components|DestroyComponent _returnvalue))
            (:Is%20Not%20Valid
              _))
          (bind _output_get_3 (LocalVariables|SetData (Utilities|Struct|MakeAttachData (.impactposition (LocalVariables|GetData)) (.impactnormal (LocalVariables|GetData)) (.attachto (LocalVariables|GetData)) (.distance (LocalVariables|GetData)) (Actor|GetComponentbyClass "/Script/Engine.StaticMeshComponent"))))
          (CallFunction|Attach _output_get_3)
          (bind _asquest_object (Utilities|Casting|CastToQuestObject (.attachto (LocalVariables|GetData))))
          (Default|AttachedtoSomething _asquest_object self)
          (else
            (CallFunction|Projection (LocalVariables|GetData))))
        (Collision|SetCollisionObjectType _staticmesh "ECC_WorldStatic")
        (Class|PrimitiveComponent|PutRigidBodytoSleep _staticmesh "None")))))

(fn EvaluateSockets)

(fn Projection
  (params (Attachment :type Attach%20Data%20Structure))
  (Utilities|IsValid (.from Attachment)
    (:Is%20Valid
      (Transformation|SetRelativeLocationAndRotation (.from Attachment) (.impactposition Attachment) (Math|Conversions|RotationFromXVector (.impactnormal Attachment)) false false))))

(fn Attach
  (params (Attachment :type Attach%20Data%20Structure))
  (Transformation|SetActorLocationAndRotation (Components|GetOwner (.from Attachment)) (.impactposition Attachment) (Math|Conversions|RotationFromXVector (.impactnormal Attachment))))