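; BP_Player is the player character, with Enhanced Input movement, pitch-clamped camera look, a weaker double jump and object grabbing.
; While falling, move input uses full forward scale and halved strafe, and landing re-arms the double jump.
; Grab line-traces from the camera for an InteractableObject and holds it with a PhysicsHandle, whose target Tick derives from a Sphere component's transform.
; Releasing grab drops the object and calls its Attatch.
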(event OnComponentBeginOverlap(Sphere)
  (params (OverlappedComponent :type Primitive%20Component%20Object%20Reference) (OtherActor :type Actor%20Object%20Reference) (OtherComp :type Primitive%20Component%20Object%20Reference) (OtherBodyIndex :type Integer) (bFromSweep :type Boolean) (SweepResult :type Hit%20Result%20Structure%20%28by%20ref%29))
  ;[1 1 1] Indicate if object is pick-up-able
  (if (Actor|ActorHasTag OtherActor "PickUp")
    _))

(event Input|EnhancedActionEvents|EnhancedInputActionIA_Move
  (params (ActionValue :type Vector%202D%20Structure) (ElapsedSeconds :type Float%20%28double-precision%29) (TriggeredSeconds :type Float%20%28double-precision%29) (InputAction :type Input%20Action%20Object%20Reference :default "/Game/FirstPerson/Input/Actions/IA_Move.IA_Move"))
  (bind _camera (Variables|Default|GetCamera))
  (bind _charactermovement (Variables|Character|GetCharacterMovement))
  (bind _returnvalue (AI|Components|NavMovement|IsFalling _charactermovement))
  (Pawn|Input|AddMovementInput (Math|Vector|GetForwardVector _camera) (Math|Float|SelectFloat 1.0 (.y ActionValue) _returnvalue) false)
  (Pawn|Input|AddMovementInput (Math|Vector|GetRightVector _camera) (Math|Float|SelectFloat (* (.x ActionValue) 0.5) (.x ActionValue) _returnvalue) false))

(event Input|EnhancedActionEvents|EnhancedInputActionIA_Look
  (params (ActionValue :type Vector%202D%20Structure) (ElapsedSeconds :type Float%20%28double-precision%29) (TriggeredSeconds :type Float%20%28double-precision%29) (InputAction :type Input%20Action%20Object%20Reference :default "/Game/FirstPerson/Input/Actions/IA_Look.IA_Look"))
  (bind _camera (Variables|Default|GetCamera))
  (bind _relativerotation (Variables|/Script/Engine.SceneComponent|GetRelativeRotation _camera))
  (Transformation|AddRelativeRotation _camera (Math|Rotator|MakeRotator 0.0 (* (.y ActionValue) (Variables|Default|GetCameraYSensitivity)) (* (.x ActionValue) (Variables|Default|GetCameraXSensitivity))) false false)
  (if (> (.pitch _relativerotation) 8e+01)
    (Transformation|SetRelativeRotation _camera (Math|Rotator|MakeRotator (.roll _relativerotation) 8e+01 (.yaw _relativerotation)) false false)
    (elif (< (.pitch _relativerotation) -8e+01)
      (Transformation|SetRelativeRotation _camera (Math|Rotator|MakeRotator (.roll _relativerotation) -8e+01 (.yaw _relativerotation)) false false))))

(event Input|EnhancedActionEvents|EnhancedInputActionIA_Jump
  (params (ActionValue :type Boolean) (ElapsedSeconds :type Float%20%28double-precision%29) (TriggeredSeconds :type Float%20%28double-precision%29) (InputAction :type Input%20Action%20Object%20Reference :default "/Game/FirstPerson/Input/Actions/IA_Jump.IA_Jump"))
  (bind _charactermovement (Variables|Character|GetCharacterMovement))
  (:Started
    (if (AI|Components|NavMovement|IsFalling (Variables|Character|GetCharacterMovement))
      (if (Variables|Default|GetCanDJump)
        (Utilities|FlowControl|DoOnce false
          (:Completed
            (Variables|Default|SetCanDJump false)
            (Variables|/Script/Engine.CharacterMovementComponent|SetJumpZVelocity _charactermovement 1e+02)
            (Character|Jump)
            (Variables|/Script/Engine.CharacterMovementComponent|SetJumpZVelocity _charactermovement 2e+02)
            (Audio|PlaySoundatLocation 0 (Transformation|GetWorldLocation (Variables|Collision|GetCapsuleComponent)) "0, 0, 0" 1.0 1.0 0.0 0 0 0 0))))
      (else
        (Character|Jump)
        (Audio|PlaySoundatLocation 0 (Transformation|GetWorldLocation (Variables|Collision|GetCapsuleComponent)) "0, 0, 0" 1.0 1.0 0.0 0 0 0 0)))))

(event Input|EnhancedActionEvents|EnhancedInputActionIA_Grab
  (params (ActionValue :type Boolean) (ElapsedSeconds :type Float%20%28double-precision%29) (TriggeredSeconds :type Float%20%28double-precision%29) (InputAction :type Input%20Action%20Object%20Reference :default "/Game/FirstPerson/Input/Actions/IA_Grab.IA_Grab"))
  (:Completed
    (Physics|Components|PhysicsHandle|ReleaseComponent (Variables|Default|GetPhysicsHandle))
    (Variables|Default|SetIsHoldingObject false)
    (Utilities|IsValid (Variables|Default|GetPickedUpActor)
      (:Is%20Valid
        (bind _asinteractable_object (Utilities|Casting|CastToInteractableObject (Variables|Default|GetPickedUpActor)))
        (Default|Attatch _asinteractable_object)
        (Variables|Default|SetPickedUpActor 0)))))

(event Input|EnhancedActionEvents|EnhancedInputActionIA_Grab
  (params (ActionValue :type Boolean) (ElapsedSeconds :type Float%20%28double-precision%29) (TriggeredSeconds :type Float%20%28double-precision%29) (InputAction :type Input%20Action%20Object%20Reference :default "/Game/FirstPerson/Input/Actions/IA_Grab.IA_Grab"))
  (bind _camera (Variables|Default|GetCamera))
  (bind _returnvalue (Transformation|GetWorldLocation _camera))
  (:Started
    (if (not (Variables|Default|GetIsHoldingObject))
      (bind _outhit (Collision|LineTraceByChannel _returnvalue (+ _returnvalue (* (Math|Vector|GetForwardVector _camera) 1.5e+02)) "TraceTypeQuery1" false 0 "Persistent"))
      (bind _asinteractable_object (Utilities|Casting|CastToInteractableObject (.HitActor (Collision|BreakHitResult _outhit))))
      (Utilities|IsValid _asinteractable_object
        (:Is%20Valid
          (Variables|Default|SetPickedUpActor _asinteractable_object)
          (Physics|Components|PhysicsHandle|GrabComponentatLocationwithRotation (Variables|Default|GetPhysicsHandle) (.HitComponent (Collision|BreakHitResult _outhit)) "None" (.ImpactPoint (Collision|BreakHitResult _outhit)) "0, 0, 0")
          (Class|PrimitiveComponent|WakeRigidBody (.HitComponent (Collision|BreakHitResult _outhit)) "None")
          (Variables|Default|SetIsHoldingObject true)
          (Default|Grabbed (Variables|Default|GetPickedUpActor)))))))

(event EventBeginPlay
  (bind _returnvalue (Game|GetPlayerCameraManager 0))
  (bind _asplayer_controller (Utilities|Casting|CastToPlayerController (Pawn|GetController)))
  (Input|AddMappingContext (PlayerController|LocalPlayerSubsystems|GetEnhancedInputLocalPlayerSubsystem _asplayer_controller) "/Game/FirstPerson/Input/IMC_TapeDuck.IMC_TapeDuck" 0 "(bIgnoreAllPressedKeysUntilRelease=True,bForceImmediately=False,bNotifyUserSettings=False)")
  (Variables|/Script/Engine.PlayerCameraManager|SetViewPitchMax _returnvalue 7e+01)
  (Variables|/Script/Engine.PlayerCameraManager|SetViewPitchMin _returnvalue -7e+01))

(event Collision|EventActorBeginOverlap
  (params (OtherActor :type Actor%20Object%20Reference)))

(event EventTick
  (params (DeltaSeconds :type Float%20%28single-precision%29))
  (bind _physicshandle (Variables|Default|GetPhysicsHandle))
  (bind _sphere (Variables|Default|GetSphere))
  (bind _returnvalue (Transformation|GetWorldTransform _sphere))
  (Class|PhysicsHandleComponent|SetTargetLocationandRotation _physicshandle (Math|Interpolation|VInterpTo (.location _returnvalue) (.TargetLocation (Class|PhysicsHandleComponent|GetTargetLocationandRotation _physicshandle)) DeltaSeconds 1.0) (.rotation _returnvalue)))

(event EventOnLanded
  (params (Hit :type Hit%20Result%20Structure%20%28by%20ref%29))
  (bind _charactermovement (Variables|Character|GetCharacterMovement))
  (Variables|Default|SetCanDJump true)
  (Utilities|FlowControl|DoOnce false) ; enters at Reset
)

(fn ConstructionScript)