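; Seesaw actor that tests whether an actor passed to it counts as heavy, apparently an unfinished gameplay prop.
; CheckFit scans that actor's tags for "Heavy" and latches IsHeavy, which is never cleared here.
; When IsHeavy is set it only prints a debug string, with a note about replacing placeholder feedback with animation.
; EchoType always returns true, and the construction script only calls its parent.
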(event EventBeginPlay
  (|CallParentFunction) ; This node is disabled and will not be called.\nDrag off pins to build functionality.
)

(event Collision|EventActorBeginOverlap
  (params (OtherActor :type Actor%20Object%20Reference))
  (|CallParentFunction OtherActor) ; This node is disabled and will not be called.\nDrag off pins to build functionality.
)

(event EventTick
  (params (DeltaSeconds :type Float%20%28single-precision%29))
  (|CallParentFunction DeltaSeconds) ; This node is disabled and will not be called.\nDrag off pins to build functionality.
)

(event EventCheckFit
  (params (From :type Interactable%20Object%20Object%20Reference))
  (bind _array_element (Utilities|Array|ForEachLoopwithBreak (Variables|/Script/Engine.Actor|GetTags From) :!label _label)
    (:LoopBody
      (if (== "Heavy" _array_element)
        (Variables|Default|SetIsHeavy (== "Heavy" _array_element))
        (goto _label Break)))
    (:Completed
      ;[1 1 1] Replace play sound 2d with animation
      (if (Variables|Default|GetIsHeavy)
        (Development|PrintString "Hello")))))

(fn ConstructionScript
  (|CallParentFunction))

(fn EchoType
  (return true))