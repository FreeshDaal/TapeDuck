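; Rocket actor that counts matching objects passed to it and triggers a rocket video once it has enough.
; CheckFit passes the sender to AddToObject, which increments a counter when the sender's EchoType message returns true, printing debug text.
; From the second match onward, it stops the player's movement and adds a RocketVideo widget to the viewport.
; The rocket's own EchoType returns false.
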(event EventBeginPlay)

(event Collision|EventActorBeginOverlap
  (params (OtherActor :type Actor%20Object%20Reference)))

(event EventTick
  (params (DeltaSeconds :type Float%20%28single-precision%29)))

(event EventCheckFit
  (params (From :type Interactable%20Object%20Object%20Reference))
  (CallFunction|AddtoObject From))

(event EventAnimation
  ;[1 1 1] Play animation here
  (CallFunction|StopPlayer)
  (bind _returnvalue (UserInterface|CreateWidget "/Game/UI/RocketShit/RocketVideo.RocketVideo_C" (Game|GetPlayerController 0)))
  (UserInterface|Viewport|AddtoViewport _returnvalue 0))

(fn ConstructionScript)

(fn AddtoObject
  (params (Test :type Actor%20Object%20Reference))
  (bind _isoftype (Class|QuestObjects|EchoType(Message) Test))
  (bind _output_get (LocalVariables|SetisOfType _isoftype))
  (if _output_get
    (bind _output_get_2 (Variables|Default|SetObjects (+ (Variables|Default|GetObjects) 1)))
    (if (>= _output_get_2 2)
      (Development|PrintString "Hello")
      (CallFunction|Animation)
      (else
        (Development|PrintString "not yet")))))

(fn StopPlayer
  (AI|Navigation|StopMovement (Game|GetPlayerController 0)))

(fn EchoType
  (return false))